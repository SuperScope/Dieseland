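; UIPlayerController is a player controller that, by its name, serves the user interface.
; Pressing the UpgradeDexterity action sets the click trace channel to WorldStatic, its only active logic.
; MoveRight and MoveForward axis events are empty.
; Disconnected logic would nudge the mouse cursor horizontally or vertically in fixed pixel steps by axis sign, using ViewportSetMousePosition, but never runs.
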(event `InputAction|UpgradeDexterity`
  (:`Pressed`
    (set `self.CurrentClickTraceChannel` "ECC_WorldStatic")))

(event `InputAxis|MoveRight`
  (params (AxisValue :type "Float (single-precision)")))

(event `InputAxis|MoveForward`
  (params (AxisValue :type "Float (single-precision)")))

(fn `UserConstructionScript`)