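; HUD Blueprint for Dieseland that shows the player character's skill cooldowns, ammo, reload timer and collected scrap.
; BeginPlay creates the DieselandHUDView widget and attempts to cache the character, though that cast has no pawn wired in.
; DrawHUD pushes character values into the widget's text fields every frame.
; ShowLevels sets Constitution, Strength and Dexterity text but is never called here, and its Intelligence update is disconnected.
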(event `self.ReceiveBeginPlay`
  (bind _returnvalue (`WidgetBlueprintLibrary.Create` "/Game/Blueprints/UserInterface/DieselandHUDView.DieselandHUDView_C"))
  (`UserWidget.AddToViewport` _returnvalue false false false)
  (bind _asdieselandhudview_c (cast `/Game/Blueprints/UserInterface/DieselandHUDView` _returnvalue))
  (set `self.DieselandHUDView` _asdieselandhudview_c)
  (bind _asdieselandplayercontroller (cast `DieselandPlayerController` (`self.GetOwningPlayerController`)))
  (bind _asdieselandcharacter (cast `DieselandCharacter` null))
  (set `self.DieselandCharacter` _asdieselandcharacter))

(event `self.ReceiveDrawHUD`
  (params (SizeX :type Integer) (SizeY :type Integer))
  (`self.ShowSkillCooldowns`)
  (`self.ShowResources`))

(fn `ShowLevels`
  (bind _dieselandcharacter (`self.DieselandCharacter`))
  (bind _dieselandhudview (`self.DieselandHUDView`))
  (`TextBlock.SetText` (`/Game/Blueprints/UserInterface/DieselandHUDView.Con Lvl` _dieselandhudview) (`KismetTextLibrary.Conv_IntToText` (`DieselandCharacter.Constitution` _dieselandcharacter) "HalfToEven"))
  (`TextBlock.SetText` (`/Game/Blueprints/UserInterface/DieselandHUDView.Str Lvl` _dieselandhudview) (`KismetTextLibrary.Conv_IntToText` (`DieselandCharacter.Strength` _dieselandcharacter) "HalfToEven"))
  (`TextBlock.SetText` (`/Game/Blueprints/UserInterface/DieselandHUDView.Dex Lvl` _dieselandhudview) (`KismetTextLibrary.Conv_IntToText` (`DieselandCharacter.Dexterity` _dieselandcharacter) "HalfToEven")))

(fn `ShowResources`
  (bind _dieselandcharacter (`self.DieselandCharacter`))
  (bind _dieselandhudview (`self.DieselandHUDView`))
  (`TextBlock.SetText` (`/Game/Blueprints/UserInterface/DieselandHUDView.Ammo Remaining` _dieselandhudview) (`KismetTextLibrary.Conv_IntToText` (`DieselandCharacter.BasicAttackAmmo` _dieselandcharacter) "HalfToEven"))
  (`TextBlock.SetText` (`/Game/Blueprints/UserInterface/DieselandHUDView.Reload Cooldown` _dieselandhudview) (`KismetTextLibrary.Conv_DoubleToText` (`DieselandCharacter.BasicAttackReloadTimer` _dieselandcharacter) "HalfToEven"))
  (`TextBlock.SetText` (`/Game/Blueprints/UserInterface/DieselandHUDView.Scrap Collected` _dieselandhudview) (`KismetTextLibrary.Conv_IntToText` (`DieselandCharacter.Scrap` _dieselandcharacter) "HalfToEven")))

(fn `ShowSkillCooldowns`
  (bind _dieselandcharacter (`self.DieselandCharacter`))
  (bind _dieselandhudview (`self.DieselandHUDView`))
  (`TextBlock.SetText` (`/Game/Blueprints/UserInterface/DieselandHUDView.Skill 1 Cooldown` _dieselandhudview) (`KismetTextLibrary.Conv_DoubleToText` (`DieselandCharacter.SkillOneTimer` _dieselandcharacter) "HalfToEven"))
  (`TextBlock.SetText` (`/Game/Blueprints/UserInterface/DieselandHUDView.Skill 2 Cooldown` _dieselandhudview) (`KismetTextLibrary.Conv_DoubleToText` (`DieselandCharacter.SkillTwoTimer` _dieselandcharacter) "HalfToEven"))
  (`TextBlock.SetText` (`/Game/Blueprints/UserInterface/DieselandHUDView.Skill 3 Cooldown` _dieselandhudview) (`KismetTextLibrary.Conv_DoubleToText` (`DieselandCharacter.SkillThreeTimer` _dieselandcharacter) "HalfToEven")))

(fn `UserConstructionScript`)