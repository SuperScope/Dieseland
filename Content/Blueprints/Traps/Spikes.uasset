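; Spike trap actor that repeatedly sinks its Spikes component slowly and thrusts it back up quickly, driven only on the server.
; On authority, BeginPlay caches up and down positions and plays the Spike_Move timeline to lerp between them.
; Tick also moves the same component, using a CanTick gate around latent MoveComponentTo calls and a delay to loop the lower-and-raise cycle.
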(event `self.ReceiveBeginPlay`
  (bind _relativelocation (`SceneComponent.RelativeLocation` (`self.Spikes`)))
  (`/Engine/EditorBlueprintResources/ActorMacros.Switch Has Authority`
    (:`Authority`
      (set `self.UpLocation` _relativelocation)
      (set `self.DownLocation` (+ (0.0 0.0 -60.0) _relativelocation))
      (bind (_direction _newtrack_1) (`Timeline|Spike_Move`)
        (:`Update`
          (`SceneComponent.SetRelativeLocation` (`self.Spikes`) (`KismetMathLibrary.VLerp` (`self.DownLocation`) (`self.UpLocation`) _newtrack_1) false))))))

(event `self.ReceiveTick`
  (params (DeltaSeconds :type "Float (single-precision)"))
  (bind _spikes (`self.Spikes`))
  (bind _spikes_2 (`self.Spikes`))
  (`/Engine/EditorBlueprintResources/ActorMacros.Switch Has Authority`
    (:`Authority`
      (if (`self.CanTick`)
        (set `self.CanTick` false)
        (`KismetSystemLibrary.MoveComponentTo` _spikes_2 (`KismetMathLibrary.MakeVector` (.x (`SceneComponent.RelativeLocation` _spikes_2)) (.y (`SceneComponent.RelativeLocation` _spikes_2)) (+ (.z (`SceneComponent.RelativeLocation` _spikes_2)) -60.0)) (`SceneComponent.RelativeRotation` _spikes_2) false false 2.5)
        (`KismetSystemLibrary.Delay` 3.0)
        (`KismetSystemLibrary.MoveComponentTo` _spikes (`KismetMathLibrary.MakeVector` (.x (`SceneComponent.RelativeLocation` _spikes)) (.y (`SceneComponent.RelativeLocation` _spikes)) (+ (.z (`SceneComponent.RelativeLocation` _spikes)) 60.0)) (`SceneComponent.RelativeRotation` _spikes) false false 0.5)
        (set `self.CanTick` true)))))

(fn `UserConstructionScript`)