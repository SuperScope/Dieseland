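; Oil trap that periodically switches on a rotating particle effect and its collision.
; A Tick event gated by the CanTick flag waits out a short delay, then activates the particles and sets collision to overlap all channels.
; The Oil_Rotate timeline spins the particles through nearly a full turn, then deactivates them, ignores all collision and re-arms the flag to repeat the cycle.
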(event `self.ReceiveTick`
  (params (DeltaSeconds :type "Float (single-precision)"))
  (if (`self.CanTick`)
    (set `self.CanTick` false)
    (`KismetSystemLibrary.Delay` null 3.0)
    (`ActorComponent.SetActive` (`self.ParticleSystem1`) true false)
    (`PrimitiveComponent.SetCollisionResponseToAllChannels` (`self.Collision`) "ECR_Overlap")
    (bind (_direction _newtrack_0) (`Timeline|Oil_Rotate` :!via `PlayFromStart`)
      (:`Update`
        (`SceneComponent.SetWorldRotation` (`self.ParticleSystem1`) (`KismetMathLibrary.RLerp` (struct :`Roll` 90.0) (struct :`Yaw` 359.0 :`Roll` 90.0) _newtrack_0) false))
      (:`Finished`
        (`ActorComponent.SetActive` (`self.ParticleSystem1`) false false)
        (`PrimitiveComponent.SetCollisionResponseToAllChannels` (`self.Collision`) "ECR_Ignore")
        (set `self.CanTick` true)))))

(fn `UserConstructionScript`)