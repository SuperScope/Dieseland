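; Fire trap Blueprint that switches a flame particle effect and its box collision on and off in a repeating cycle.
; Tick uses a CanTick gate to start each cycle, with delays holding the fire off for three seconds and on for two.
; Box1 responds with Overlap to all channels while the particles are active and Ignore otherwise; no damage logic appears here.
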(event `self.ReceiveTick`
  (params (DeltaSeconds :type "Float (single-precision)"))
  (if (`self.CanTick`)
    (set `self.CanTick` false)
    (`KismetSystemLibrary.Delay` null 3.0)
    (`ActorComponent.SetActive` (`self.ParticleSystem1`) true false)
    (`PrimitiveComponent.SetCollisionResponseToAllChannels` (`self.Box1`) "ECR_Overlap")
    (`KismetSystemLibrary.Delay` null 2.0)
    (`ActorComponent.SetActive` (`self.ParticleSystem1`) false false)
    (`PrimitiveComponent.SetCollisionResponseToAllChannels` (`self.Box1`) "ECR_Ignore")
    (set `self.CanTick` true)))

(fn `UserConstructionScript`)