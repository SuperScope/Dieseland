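; Player controller Blueprint for Dieseland that toggles the in-game menu when the InGameMenu input action is pressed.
; Opening shows the mouse cursor and creates fresh overlay and menu widgets, adding the overlay to the viewport before the menu.
; Closing hides the cursor and removes both widgets, with a boolean tracking whether the menu is showing.
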(event `InputAction|InGameMenu`
  (:`Pressed`
    (if (`self.InGameMenuShowing`)
      (set `self.bShowMouseCursor` false)
      (`UserWidget.RemoveFromViewport` (`self.InGameMenuOverlay`))
      (set `self.InGameMenuShowing` false)
      (`UserWidget.RemoveFromViewport` (`self.InGameMenu`))
      (else
        (set `self.bShowMouseCursor` true)
        (bind _returnvalue (`|CreateWidget` "/Game/Blueprints/UserInterface/InGameMenuOverlay.InGameMenuOverlay_C"))
        (`UserWidget.AddToViewport` _returnvalue)
        (set `self.InGameMenuOverlay` _returnvalue)
        (set `self.InGameMenuShowing` true)
        (bind _returnvalue_2 (`|CreateWidget` "/Game/Blueprints/UserInterface/InGameMenu.InGameMenu_C"))
        (`UserWidget.AddToViewport` _returnvalue_2)
        (set `self.InGameMenu` _returnvalue_2)))))

(fn `UserConstructionScript`)