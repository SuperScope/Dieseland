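; DeathTileBP is a level tile that rises on BeginPlay and drops back down once no enemies remain.
; Two timelines lerp the actor's location vertically by a fixed offset, updating IsTileDown as each finishes.
; Between moves it clears ReadyToRise and loops on EnemiesRemaining with no delay in the loop.
; After the descent it calls SwitchDeathTile, whose logic is not defined here.
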(event `self.ReceiveBeginPlay`
  (bind _returnvalue (`self.K2_GetActorLocation`))
  (bind _returnvalue_2 (`self.K2_GetActorLocation`))
  (set `self.CurrentLocation` _returnvalue_2)
  (set `self.TargetLocation` (`KismetMathLibrary.MakeVector` (.x _returnvalue_2) (.y _returnvalue_2) (+ (.z _returnvalue_2) 1500.0)))
  (bind (_direction _tile_raise_drop) (`Timeline|TileMovementUp` :!via `PlayFromStart`)
    (:`Update`
      (`self.K2_SetActorLocation` (`KismetMathLibrary.VLerp` (`self.CurrentLocation`) (`self.TargetLocation`) _tile_raise_drop)))
    (:`Finished`
      (set `self.IsTileDown` false)
      (set `self.ReadyToRise` false :!label _label)
      (if (`self.EnemiesRemaining`)
        (goto _label)
        (else
          (set `self.CurrentLocation` _returnvalue)
          (set `self.TargetLocation` (`KismetMathLibrary.MakeVector` (.x _returnvalue) (.y _returnvalue) (+ (.z _returnvalue) -1500.0)))
          (bind (_direction_2 _tile_raise_drop_2) (`Timeline|TileMovementDown` :!via `PlayFromStart`)
            (:`Update`
              (`self.K2_SetActorLocation` (`KismetMathLibrary.VLerp` (`self.CurrentLocation`) (`self.TargetLocation`) _tile_raise_drop_2)))
            (:`Finished`
              (set `self.IsTileDown` true)
              (`self.SwitchDeathTile`))))))))

(fn `UserConstructionScript`)