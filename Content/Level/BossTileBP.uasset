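; Boss arena tile that runs a King or Queen encounter, chosen by BossTag.
; When Spawn is set, it spawns the boss with four minions and signals zone-tagged gates that the fight started.
; While CheckForBoss is set, a delayed Tick poll searches overlapping actors for the boss class.
; If none is found, it flags BossDead, finishes the gates, teleports players and sets Teleport on bridge tiles matching BossTag.
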(event `self.ReceiveBeginPlay`
  (bind _outactors (`GameplayStatics.GetAllActorsOfClass` "/Game/Level/BossGates/Gate1.Gate1_C"))
  (set `self.BossGates` _outactors)
  (bind _outactors_2 (`GameplayStatics.GetAllActorsOfClass` "/Game/Level/BridgeTileBP.BridgeTileBP_C"))
  (set `self.BridgeTiles` _outactors_2)
  (bind _outactors_3 (`GameplayStatics.GetAllActorsOfClass` "/Game/Level/BridgeTileCornerBP.BridgeTileCornerBP_C"))
  (set `self.BridgeCornerTile` _outactors_3))

(event `self.ReceiveTick`
  (params (DeltaSeconds :type "Float (single-precision)"))
  (`|ExecutionSequence`
    (:`then_0`
      (if (`self.CheckForBoss`)
        (if (`self.ActorHasTag` (`self.ZoneTag`))
          (set `self.IsBossAlive` false)
          (`KismetSystemLibrary.Delay` 4.0)
          (for _array_element (`self.GetOverlappingActors` null)
            (if (== (`self.BossTag`) "King")
              (bind _returnvalue (`GameplayStatics.GetObjectClass` _array_element))
              (if (== _returnvalue "/Game/Blueprints/Enemies/DieselandHighLanderKingBP.DieselandHighLanderKingBP_C")
                (set `self.IsBossAlive` true :!label _label))
              (elif (== _returnvalue "/Game/Blueprints/Enemies/DieselandWalkerQueenBP.DieselandWalkerQueenBP_C")
                (goto _label))))
          (if (not (`self.IsBossAlive`))
            (set `self.CheckForBoss` false)
            (`KismetSystemLibrary.Delay` 15.0)
            (set `self.BossDead` true)
            (for _array_element_2 (`self.BossGates`)
              (if (`self.ActorHasTag` _array_element_2 (`self.ZoneTag`))
                (bind _asgate1_c (cast `/Game/Level/BossGates/Gate1` _array_element_2))
                (set `BossTiles.BossFinish` true _asgate1_c)
                (`KismetSystemLibrary.Delay` 5.0)
                (`|ExecutionSequence`
                  (:`then_0`
                    (set `self.PlayerArray` (`self.GetOverlappingActors` null))
                    (`self.TeleportPlayers`))
                  (:`then_1`
                    (for _array_element_3 (`self.BridgeTiles`)
                      (if (`self.ActorHasTag` _array_element_3 (`self.BossTag`))
                        (bind _asbridgetilebp_c (cast `/Game/Level/BridgeTileBP` _array_element_3))
                        (set `BossTiles.Teleport` true _asbridgetilebp_c))))
                  (:`then_2`
                    (for _array_element_4 (`self.BridgeCornerTile`)
                      (if (`self.ActorHasTag` _array_element_4 (`self.BossTag`))
                        (bind _asbridgetilecornerbp_c (cast `/Game/Level/BridgeTileCornerBP` _array_element_4))
                        (set `BossTiles.Teleport` true _asbridgetilecornerbp_c)))))))))))
    (:`then_1`
      (if (`self.ActorHasTag` (`self.ZoneTag`))
        (if (`self.Spawn`)
          (`self.SpawnBoss`))))))

(event `SpawnBoss`
  (bind _returnvalue (`SceneComponent.K2_GetComponentLocation` (`self.EnemySpawn4`)))
  (bind _returnvalue_2 (`SceneComponent.K2_GetComponentLocation` (`self.BossSpawn`)))
  (bind _returnvalue_3 (`SceneComponent.K2_GetComponentLocation` (`self.EnemySpawn1`)))
  (bind _returnvalue_4 (`SceneComponent.K2_GetComponentLocation` (`self.EnemySpawn2`)))
  (bind _returnvalue_5 (`SceneComponent.K2_GetComponentLocation` (`self.EnemySpawn3`)))
  (set `self.Spawn` false)
  (if (== (`self.BossTag`) "King")
    (`AIBlueprintHelperLibrary.SpawnAIFromClass` "/Game/Blueprints/Enemies/DieselandHighLanderKingBP.DieselandHighLanderKingBP_C" "/Game/BehaviorTrees/NeutralAggressiveEnemyBehaviorTree.NeutralAggressiveEnemyBehaviorTree" _returnvalue_2)
    (`AIBlueprintHelperLibrary.SpawnAIFromClass` "/Game/Blueprints/Enemies/DieselandHighlanderBP.DieselandHighlanderBP_C" "/Game/BehaviorTrees/NeutralAggressiveEnemyBehaviorTree.NeutralAggressiveEnemyBehaviorTree" _returnvalue_3)
    (`AIBlueprintHelperLibrary.SpawnAIFromClass` "/Game/Blueprints/Enemies/DieselandHighlanderBP.DieselandHighlanderBP_C" "/Game/BehaviorTrees/NeutralAggressiveEnemyBehaviorTree.NeutralAggressiveEnemyBehaviorTree" _returnvalue_4)
    (`AIBlueprintHelperLibrary.SpawnAIFromClass` "/Game/Blueprints/Enemies/DieselandHighlanderBP.DieselandHighlanderBP_C" "/Game/BehaviorTrees/NeutralAggressiveEnemyBehaviorTree.NeutralAggressiveEnemyBehaviorTree" _returnvalue_5)
    (`AIBlueprintHelperLibrary.SpawnAIFromClass` "/Game/Blueprints/Enemies/DieselandHighlanderBP.DieselandHighlanderBP_C" "/Game/BehaviorTrees/NeutralAggressiveEnemyBehaviorTree.NeutralAggressiveEnemyBehaviorTree" _returnvalue)
    (else
      (`AIBlueprintHelperLibrary.SpawnAIFromClass` "/Game/Blueprints/Enemies/DieselandWalkerQueenBP.DieselandWalkerQueenBP_C" "/Game/BehaviorTrees/NeutralAggressiveEnemyBehaviorTree.NeutralAggressiveEnemyBehaviorTree" _returnvalue_2)
      (`AIBlueprintHelperLibrary.SpawnAIFromClass` "/Game/Blueprints/Enemies/DieselandWalkerBP.DieselandWalkerBP_C" "/Game/BehaviorTrees/NeutralAggressiveEnemyBehaviorTree.NeutralAggressiveEnemyBehaviorTree" _returnvalue_3)
      (`AIBlueprintHelperLibrary.SpawnAIFromClass` "/Game/Blueprints/Enemies/DieselandWalkerBP.DieselandWalkerBP_C" "/Game/BehaviorTrees/NeutralAggressiveEnemyBehaviorTree.NeutralAggressiveEnemyBehaviorTree" _returnvalue_4)
      (`AIBlueprintHelperLibrary.SpawnAIFromClass` "/Game/Blueprints/Enemies/DieselandWalkerBP.DieselandWalkerBP_C" "/Game/BehaviorTrees/NeutralAggressiveEnemyBehaviorTree.NeutralAggressiveEnemyBehaviorTree" _returnvalue_5)
      (`AIBlueprintHelperLibrary.SpawnAIFromClass` "/Game/Blueprints/Enemies/DieselandWalkerBP.DieselandWalkerBP_C" "/Game/BehaviorTrees/NeutralAggressiveEnemyBehaviorTree.NeutralAggressiveEnemyBehaviorTree" _returnvalue)))
  (for _array_element (`self.BossGates`)
    (if (`self.ActorHasTag` _array_element (`self.ZoneTag`))
      (bind _asgate1_c (cast `/Game/Level/BossGates/Gate1` _array_element))
      (set `BossTiles.BossStart` true _asgate1_c))))

(fn `UserConstructionScript`)