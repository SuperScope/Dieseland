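; Base death tile Blueprint that rises into the level, spawns enemy bots, and sinks again once none remain.
; BeginPlay raises it by timeline lerp, then spawns Walkers or Highlander Kings based on component-name substrings; only Walkers receive their component's transform.
; After a delay, Tick polls for remaining enemies, then a second timeline lowers the tile and calls SwitchDeathTile.
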(event `self.ReceiveBeginPlay`
  (bind _returnvalue (`self.K2_GetActorLocation`))
  ;[0.1807 1 0.003757] Move up on start
  (set `self.CurrentLocation` _returnvalue)
  (set `self.TargetLocation` (`KismetMathLibrary.MakeVector` (.x _returnvalue) (.y _returnvalue) (+ (.z _returnvalue) 1555.0)))
  (bind (_direction _raise_lower) (`Timeline|TileMovementUp` :!via `PlayFromStart`)
    (:`Update`
      (`self.K2_SetActorLocation` (`KismetMathLibrary.VLerp` (`self.CurrentLocation`) (`self.TargetLocation`) _raise_lower)))
    (:`Finished`
      ;[0.3967 0.3238 1] Spawn actors at correct locations
      (for _array_element (`self.K2_GetComponentsByClass` "/Script/Engine.SceneComponent")
        (bind _asscenecomponent (cast `SceneComponent` _array_element))
        (bind _returnvalue_2 (`KismetSystemLibrary.GetDisplayName` _asscenecomponent))
        (if (> (`KismetStringLibrary.FindSubstring` _returnvalue_2 "Walker") 0)
          (`self.SpawnBot` (`SceneComponent.K2_GetComponentToWorld` _asscenecomponent) "/Game/Blueprints/Enemies/DieselandWalkerBP.DieselandWalkerBP_C")
          (elif (> (`KismetStringLibrary.FindSubstring` _returnvalue_2 "Highlander") 0)
            (`self.SpawnBot` (struct) "/Game/Blueprints/Enemies/DieselandHighLanderKingBP.DieselandHighLanderKingBP_C"))))
      (`KismetSystemLibrary.Delay` 30.0)
      (set `self.IsTileDown` false)
      (set `self.ReadyToRise` false)
      (set `self.CheckForEnemies` true))))

(event `self.ReceiveTick`
  (params (DeltaSeconds :type "Float (single-precision)"))
  (bind _returnvalue (`self.K2_GetActorLocation`))
  ;[1 0.9834 0.1699] Move back down when no enemies present
  (if (`self.CheckForEnemies`)
    (if (not (`self.EnemiesRemaining`))
      (set `self.CheckForEnemies` false)
      (set `self.CurrentLocation` _returnvalue)
      (set `self.TargetLocation` (`KismetMathLibrary.MakeVector` (.x _returnvalue) (.y _returnvalue) (+ (.z _returnvalue) -1500.0)))
      (bind (_direction _raise_lower) (`Timeline|TileMovementDown` :!via `PlayFromStart`)
        (:`Update`
          (`self.K2_SetActorLocation` (`KismetMathLibrary.VLerp` (`self.CurrentLocation`) (`self.TargetLocation`) _raise_lower)))
        (:`Finished`
          (set `self.IsTileDown` true)
          (`self.SwitchDeathTile`))))))

(fn `SpawnBot`
  (params (Location :type "Object.Transform Structure") (EnemyType :type "Pawn Class Reference"))
  (bind _returnvalue (`|SpawnActorFromClass` EnemyType Location true))
  (bind _asdieselandenemybot (cast `DieselandEnemyBot` _returnvalue))
  (`Pawn.SpawnDefaultController` _asdieselandenemybot))

(fn `UserConstructionScript`)